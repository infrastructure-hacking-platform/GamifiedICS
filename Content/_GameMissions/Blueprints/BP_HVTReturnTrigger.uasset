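; BP_HVTReturnTrigger is a mission trigger volume that reports when the high-value target (HVT) NPC enters it.
; Its box starts without collision, and mission activate and deactivate events toggle query collision through multicasts.
; On the authority, the first overlap by a TargetNPC sends a configured mission event message to the game state and latches so it fires only once.
; Construction applies its mission tags.
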(event Custom|Multicast_Activate
  (Collision|SetCollisionEnabled (Variables|Default|GetBox) "QueryOnly"))

(event Custom|Multicast_Deactivate
  (Collision|SetCollisionEnabled (Variables|Default|GetBox) "NoCollision"))

(event EventBeginPlay)

(event Collision|EventActorBeginOverlap
  (params (OtherActor :type Actor%20Object%20Reference))
  (Utilities|Casting|CastToTargetNPC OtherActor) ; This is switched out from the regular pawn cast to check specifically for the HVT actor
  (Networking|SwitchHasAuthority
    (:Authority
      (if (not (Variables|Default|GetbTriggered))
        (Variables|Default|SetbTriggered true)
        (Class|WarwolfMissionInterface|SendMissionEvent(Message) (Game|GetGameState) (Variables|Default|GetEventToSend))))))

(event EventActivateMissionActor
  (CallFunction|MulticastActivate))

(event EventDeactivateMissionActor
  (CallFunction|MulticastDeactivate))

(fn ConstructionScript
  (Class|WarwolfMissionTagComponent|SetMissionTags (Variables|Default|GetWarwolfMissionTag) (Variables|Default|GetMissionTags))
  (Collision|SetCollisionEnabled (Variables|Default|GetBox) "NoCollision"))

(fn PlayLevelSequence
  (params (InLevelSequence :type Level%20Sequence%20Object%20Reference))
  (return 0))