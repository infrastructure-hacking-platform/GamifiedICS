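; BP_MissionTrigger is a mission actor that reports a mission event when the player enters it.
; Activate and deactivate mission actor events toggle an Activated flag that gates the trigger.
; On overlap by the player 0 pawn while active, it sends its Event value to the GameState as a mission event message.
; It has no one-shot guard, and PlayLevelSequence is an empty stub.
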(event EventActivateMissionActor
  (Variables|Default|SetActivated true))

(event EventDeactivateMissionActor
  (Variables|Default|SetActivated false))

(event Collision|EventActorBeginOverlap
  (params (OtherActor :type Actor%20Object%20Reference))
  ;[0.15 0.15 0.15 0.5] Check if Mission Activated & Player Overlaps
  (if (and (== OtherActor (Game|Player|GetPlayerPawn 0)) (Variables|Default|GetActivated))
    (Class|WarwolfMissionInterface|SendMissionEvent(Message) (Game|GetGameState) (Variables|Default|GetEvent))))

(fn ConstructionScript)

(fn PlayLevelSequence
  (params (InLevelSequence :type Level%20Sequence%20Object%20Reference))
  (return 0))