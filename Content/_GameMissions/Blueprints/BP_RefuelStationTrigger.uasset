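; BP_RefuelStationTrigger is a mission trigger box that sends the Cybertruck to the gas station when a player reaches it.
; Its collision starts disabled, and mission activate and deactivate events toggle it through multicasts.
; On the authority, a player overlap calls GoToGasStation on the first Cybertruck found and sends a mission event to the GameState, each guarded to run once.
; The construction script applies its mission tags.
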(event Custom|Multicast_Activate
  (Collision|SetCollisionEnabled (Variables|Default|GetBox) "QueryOnly"))

(event Custom|Multicast_Deactivate
  (Collision|SetCollisionEnabled (Variables|Default|GetBox) "NoCollision"))

(event EventBeginPlay)

(event Collision|EventActorBeginOverlap
  (params (OtherActor :type Actor%20Object%20Reference))
  (Utilities|Casting|CastToBP_FPMovementPlayer OtherActor) ; This looks for the player's character class
  (Networking|SwitchHasAuthority
    (:Authority
      ;[0.15 0.15 0.15 0.5] Cybertruck begins moving once player detected
      (if (Variables|Default|GetCarGone?)
        _
        (else
          (bind _outactors (Actor|GetAllActorsOfClass "/Game/EVMission/Cybertruck.Cybertruck_C"))
          (Default|GotoGasStation (Utilities|Array|Get(acopy) _outactors))
          (Variables|Default|SetCarGone? true)))
      (if (not (Variables|Default|GetbTriggered))
        (Variables|Default|SetbTriggered true)
        (Class|WarwolfMissionInterface|SendMissionEvent(Message) (Game|GetGameState) (Variables|Default|GetEventToSend))))))

(event EventActivateMissionActor
  (CallFunction|MulticastActivate))

(event EventDeactivateMissionActor
  (CallFunction|MulticastDeactivate))

(fn ConstructionScript
  (Class|WarwolfMissionTagComponent|SetMissionTags (Variables|Default|GetWarwolfMissionTag) (Variables|Default|GetMissionTags))
  (Collision|SetCollisionEnabled (Variables|Default|GetBox) "NoCollision"))

(fn PlayLevelSequence
  (params (InLevelSequence :type Level%20Sequence%20Object%20Reference))
  (return 0))