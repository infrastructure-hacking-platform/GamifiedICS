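; Game instance that manages background music, keeping the active 2D sound alive across level transitions.
; PlayMusic fades out the current player and fades in a newly created one, with events to pause, resume or stop it.
; SwitchModes reacts to playlist mode changes by playing a random track from the matching Danger, Wander, Main Menu, Defeat or Hacking playlist, with None using Wander.
; Init prepares a player with the starter cue.
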(event EventSwitchModes
  (params (New%20Mode :type Playlist_Modes%20Enum :default "NewEnumerator0"))
  ;[0.15 0.15 0.15 0.5] Music Switching logic
  (if (not (Utilities|Enum|Equal(Enum) New%20Mode (Variables|Default|GetPlaylistMode)))
    (Variables|Default|SetPlaylistMode New%20Mode)
    (CallFunction|SelectfromPlaylist(Random))))

(event EventPauseMusic
  ;[1 1 1] Stop/Resume Logic
  (Class|AudioComponent|SetPaused (Variables|Default|GetActive_Music_Player) true))

(event EventInit
  (bind _output_get (Variables|Default|SetCurrent_Track "/Game/StarterContent/Audio/Starter_Music_Cue.Starter_Music_Cue"))
  (bind _returnvalue (Audio|CreateSound2D _output_get 1.0 1.0 0.0 0 true))
  (Variables|Default|SetActive_Music_Player _returnvalue))

(event EventStopMusic
  (params (Fade%20out%20Time :type Float%20%28double-precision%29))
  ;[1 1 1] Stop Music
  (bind _output_get (Variables|Default|SetFadeOut_Music_Player_0 (Variables|Default|GetActive_Music_Player)))
  (Audio|Components|Audio|FadeOut _output_get Fade%20out%20Time 0.0 "Linear" :!class /Script/Engine.AudioComponent))

(event EventPlayMusic
  (params (Track :type Sound%20Base%20Object%20Reference) (Previous%20Track%20Fade%20out%20Time :type Float%20%28double-precision%29) (Current%20Track%20Fade%20out%20Time :type Float%20%28double-precision%29))
  ;[1 1 1] Set local vars
  (Variables|Default|SetCurrent_Track Track)
  (Variables|Default|SetPrevious%20Track%20Fade%20Out%20Time Previous%20Track%20Fade%20out%20Time)
  (Variables|Default|SetNew%20Track%20Fade%20in%20Time Current%20Track%20Fade%20out%20Time)
  (Utilities|IsValid (Variables|Default|GetActive_Music_Player)
    (:Is%20Valid
      ;[1 1 1] Fade in
      (CallFunction|StopMusic (Variables|Default|GetPrevious%20Track%20Fade%20Out%20Time)))
    (:Is%20Not%20Valid
      _))
  (bind _returnvalue (Audio|CreateSound2D (Variables|Default|GetCurrent_Track) 1.0 1.0 0.0 0 true))
  (bind _output_get (Variables|Default|SetActive_Music_Player _returnvalue))
  (Audio|Components|Audio|FadeIn _output_get (Variables|Default|GetNew%20Track%20Fade%20in%20Time) 1.0 0.0 "Linear" :!class /Script/Engine.AudioComponent))

(event EventResumeMusic
  ;[1 1 1] Stop/Resume Logic
  (Class|AudioComponent|SetPaused (Variables|Default|GetActive_Music_Player) false))

(fn SelectfromPlaylist(Random)
  (switch Utilities|FlowControl|Switch|SwitchonPlaylist_Modes (Variables|Default|GetPlaylistMode)
    (:NewEnumerator0
      (Variables|Default|SetCurrentPlaylist (Variables|Default|GetDangerPlaylist)))
    (:NewEnumerator1
      (Variables|Default|SetCurrentPlaylist (Variables|Default|GetWanderPlaylist) :!label _label))
    (:NewEnumerator2
      (Variables|Default|SetCurrentPlaylist (Variables|Default|GetMainMenuPlaylist)))
    (:NewEnumerator3
      (Variables|Default|SetCurrentPlaylist (Variables|Default|GetDefeatPlaylist)))
    (:NewEnumerator4
      (Variables|Default|SetCurrentPlaylist (Variables|Default|GetHackingPlaylist)))
    (:NewEnumerator5
      (goto _label)))
  (CallFunction|PlayMusic (.OutItem (Utilities|Array|Random (Variables|Default|GetCurrentPlaylist))) (Variables|Default|GetPrevious%20Track%20Fade%20Out%20Time) (Variables|Default|GetNew%20Track%20Fade%20in%20Time)))