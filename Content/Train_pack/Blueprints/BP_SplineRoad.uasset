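; BP_SplineRoad is a construction-time actor that builds a road by laying deforming mesh segments along its spline.
; The construction script divides the spline length by Section and adds an X-forward spline mesh component for each step.
; Each segment takes local start and end positions and tangents sampled by distance, with tangent size clamped to Section to match segment length.
; The event graph holds only disabled placeholder events, so there is no runtime logic.
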(event EventBeginPlay)

(event Collision|EventActorBeginOverlap
  (params (OtherActor :type Actor%20Object%20Reference)))

(event EventTick
  (params (DeltaSeconds :type Float%20%28single-precision%29)))

(fn ConstructionScript
  (bind _spline (Variables|Default|GetSpline))
  (bind _spline_2 (Variables|Default|GetSpline))
  ;[1 1 1] Loop and Set Mech
  (for _index (range 0 (.ReturnValue (Math|Float|Division(WholeandRemainder) (Spline|GetSplineLength (Variables|Default|GetSpline)) (Variables|Default|Getsection))))
    ;[1 1 1] This return value is the mesh that you selected to add
    (bind _returnvalue (AddComponent|AddSplineMeshComponent false))
    (SplineMesh|SetForwardAxis _returnvalue "X" true)
    (SplineMesh|SetStartandEnd _returnvalue (Spline|GetLocationatDistanceAlongSpline _spline (* _index (Variables|Default|Getsection)) "Local") (Math|Vector|ClampVectorSize (Spline|GetTangentatDistanceAlongSpline _spline (* _index (Variables|Default|Getsection)) "Local") 0.0 (Variables|Default|Getsection)) (Spline|GetLocationatDistanceAlongSpline _spline_2 (Math|Conversions|ToFloat(Integer) (+ (Math|Float|Truncate (* _index (Variables|Default|Getsection))) (Math|Float|Truncate (Variables|Default|Getsection)))) "Local") (Math|Vector|ClampVectorSize (Spline|GetTangentatDistanceAlongSpline _spline_2 (Math|Conversions|ToFloat(Integer) (+ (Math|Float|Truncate (* _index (Variables|Default|Getsection))) (Math|Float|Truncate (Variables|Default|Getsection)))) "Local") 0.0 (Variables|Default|Getsection)) true :!class /Script/Engine.SplineMeshComponent)))