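; Game state that runs the Warwolf mission system, auto-starting the prologue mission on the server at BeginPlay.
; SelectMission stores a mission data asset, loads its StateTree into the Warwolf mission manager, starts its logic and can start the mission immediately.
; StartMission sends a tagged start event to the manager after interface checks, while SendMissionEvent forwards any other StateTree event to drive the mission.
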(event EventStartMission
  ;[1 0.9309 0 0.5] Mission System
  ;;[0.15 0.15 0.15 0.5] Start Mission
  (Variables|Default|GetSelected%20Mission ; Check to see if we actually selected a mission first
    (:then
      (bind _warwolfmissionmanager (Variables|Default|GetWarwolfMissionManager)
        (:then
          (if (Utilities|DoesObjectImplementInterface _warwolfmissionmanager "/Script/WarwolfMissionSystem.WarwolfMissionInterface")
            (Class|WarwolfMissionInterface|SendMissionEvent(Message) (Variables|Default|GetWarwolfMissionManager) (Utilities|Struct|MakeStateTreeEvent "(TagName=\"Mission.Event.Start\")" "None" "BP_GamifiedICSGameState"))))
        (:else)))
    (:else
      (Development|PrintString "Mission Not Selected!"))))

(event EventSendMissionEvent
  (params (Event :type State%20Tree%20Event%20Structure%20%28by%20ref%29))
  ;[1 0.9309 0 0.5] Mission System
  ;;[0.15 0.15 0.15 0.5] Send Mission Event
  (bind _warwolfmissionmanager (Variables|Default|GetWarwolfMissionManager)
    (:then
      (Class|WarwolfMissionInterface|SendMissionEvent(Message) _warwolfmissionmanager Event))
    (:else)))

(event EventSelectMission
  (params (InMissionData :type Warwolf%20Mission%20Data%20Asset%20Object%20Reference) (bStartMissionInstantly :type Boolean))
  (bind _missionstatetree (Variables|/Script/WarwolfMissionSystem.WarwolfMissionDataAsset|GetMissionStateTree InMissionData))
  ;[1 0.9309 0 0.5] Mission System
  ;;[0.15 0.15 0.15 0.5] Select A Mission
  (Variables|Default|GetWarwolfMissionManager
    (:then
      (Utilities|IsValid _missionstatetree
        (:Is%20Valid
          (Variables|Default|SetSelected%20Mission InMissionData)
          (Class|WarwolfMissionManager|SetMissionStateTree (Variables|Default|GetWarwolfMissionManager) _missionstatetree)
          (AI|Logic|StartLogic (Variables|Default|GetWarwolfMissionManager))
          (if bStartMissionInstantly
            (Class|WarwolfMissionInterface|StartMission self)))))
    (:else)))

(event EventBeginPlay
  ;[0.1362 1 0.1094 0.5] Run Mission on Start
  (Networking|SwitchHasAuthority
    (:Authority
      (bind _missionmanager (Variables|Default|GetMissionManager)
        (:then
          (Components|Activation|Activate _missionmanager false)
          (Class|WarwolfMissionInterface|SelectMission self "/Game/_GameMissions/Prologue/DA_ICS_Prologue.DA_ICS_Prologue" true) ; The first mission is selected here (Warwolf Data Asset; Not the objective ones.)
        )
        (:else)))))

(fn ConstructionScript)