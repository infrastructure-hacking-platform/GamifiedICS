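; BP_MapMarker is a map marker component that registers itself with BP_MapManager actors as an additional layer.
; UpdateMarker, called on BeginPlay when AddOnConstruct is set, async-loads the first AdditionalLayer asset before contacting any manager.
; On completion, it finds the first manager matching each MapTag and calls UpdateAdditionalLayer with itself and the add flag.
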(event Custom|UpdateMarker
  (params (Add :type Boolean))
  (bind _values (Utilities|Map|Values (Variables|Default|GetAdditionalLayer)))
  (Utilities|AsyncLoadAsset (Utilities|Array|Get(acopy) _values)
    (:Completed
      (for _array_element (Variables|Default|GetMapTag)
        (bind _outactors (Actor|GetAllActorsOfClasswithTag "/Game/UltimateMapSystem/BPs/BP_MapManager.BP_MapManager_C" _array_element))
        (Utilities|IsValid (Utilities|Array|Get(acopy) _outactors)
          (:Is%20Valid
            (Default|UpdateAdditionalLayer (Utilities|Array|Get(acopy) _outactors) Add self)))))))

(event EventBeginPlay
  (if (Variables|Default|GetAddOnConstruct)
    (CallFunction|UpdateMarker true)))